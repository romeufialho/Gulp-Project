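; Highway traffic car that drives once along a spline path in the level and destroys itself at the end.
; On BeginPlay it picks a random mesh and finds the right or left highway path actor via IsRight, with true selecting the left path.
; A timeline moves and rotates it along the spline by distance, timed by TimeToEnd on the right path and a random duration on the left.
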(event `self.ReceiveBeginPlay`
  (`self.MoveCar`)
  (`self.RandomizeMesh`)
  (`KismetSystemLibrary.PrintString` "Spawned Left Car"))

(event `RandomizeMesh`
  (`StaticMeshComponent.SetStaticMesh` (`self.CarMesh`) (`KismetArrayLibrary.Array_Random` (`self.CarMeshes`))))

(event `MoveCar`
  (if (not (`self.IsRight?`))
    (bind _returnvalue (`GameplayStatics.GetActorOfClass` "/Game/Gulp/Blueprints/Car_Path_Highway_Right.Car_Path_Highway_Right_C"))
    (set `self.RightSplineREF` _returnvalue)
    (`self.EnterRight`)
    (else
      (bind _returnvalue_2 (`GameplayStatics.GetActorOfClass` "/Game/Gulp/Blueprints/Car_Path_Highway_Left.Car_Path_Highway_Left_C"))
      (set `self.LeftSplineREF` _returnvalue_2)
      (`self.EnterLeft`))))

(event `EnterRight`
  (bind _rightsplineref (`self.RightSplineREF`))
  (`TimelineComponent.SetPlayRate` (`self.Move1`) (/ 1.0 (`self.Time to end`)))
  (bind (_direction _move_track) (`Timeline|Move1`)
    (:`Update`
      (bind _returnvalue (`KismetMathLibrary.Lerp` 0.0 (`SplineComponent.GetSplineLength` (`/Game/Gulp/Blueprints/Car_Path_Highway_Right.Spline` (`self.RightSplineREF`))) _move_track))
      (`self.K2_SetActorTransform` (`KismetMathLibrary.MakeTransform` (`SplineComponent.GetLocationAtDistanceAlongSpline` (`/Game/Gulp/Blueprints/Car_Path_Highway_Right.Spline` _rightsplineref) _returnvalue "World") (`SplineComponent.GetRotationAtDistanceAlongSpline` (`/Game/Gulp/Blueprints/Car_Path_Highway_Right.Spline` _rightsplineref) _returnvalue "World")))
      (if (== _move_track 1.0)
        (`self.K2_DestroyActor`)))))

(event `EnterLeft`
  (bind _leftsplineref (`self.LeftSplineREF`))
  (`TimelineComponent.SetPlayRate` (`self.Move2`) (/ 1.0 (`KismetMathLibrary.RandomFloatInRange` 5.0 20.0)))
  (bind (_direction _move_track) (`Timeline|Move2`)
    (:`Update`
      (bind _returnvalue (`KismetMathLibrary.Lerp` 0.0 (`SplineComponent.GetSplineLength` (`/Game/Gulp/Blueprints/Car_Path_Highway_Left.Spline` (`self.LeftSplineREF`))) _move_track))
      (`self.K2_SetActorTransform` (`KismetMathLibrary.MakeTransform` (`SplineComponent.GetLocationAtDistanceAlongSpline` (`/Game/Gulp/Blueprints/Car_Path_Highway_Left.Spline` _leftsplineref) _returnvalue "World") (`SplineComponent.GetRotationAtDistanceAlongSpline` (`/Game/Gulp/Blueprints/Car_Path_Highway_Left.Spline` _leftsplineref) _returnvalue "World")))
      (if (== _move_track 1.0)
        (`self.K2_DestroyActor`)))))

(fn `UserConstructionScript`)