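; Game mode that runs the day loop: three clients per day over three days, tracking mood until a printed end of game.
; It spawns cars and clients at placed locations, and CheckDispatchedClients either starts the next car or adds daily mood, pauses and shows the day-end UI.
; Each client advances a daytime stage, which Tick eases toward by rotating the sky sphere.
; It also creates HUD and tutorial widgets and endlessly spawns highway traffic.
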(event `StartSpawningHighwayCars`
  (`|SpawnActorFromClass` "/Game/Gulp/Blueprints/Highway_Car_Right_BP.Highway_Car_Right_BP_C" (`KismetMathLibrary.MakeTransform` (0.0 0.0 0.0)) "Undefined" "OverrideRootScale" null null)
  (`KismetSystemLibrary.Delay` (`KismetMathLibrary.RandomFloatInRange` 0.5 5.0))
  (`|SpawnActorFromClass` "/Game/Gulp/Blueprints/Highway_Car_Left_BP.Highway_Car_Left_BP_C" (`KismetMathLibrary.MakeTransform` (0.0 0.0 0.0)) "Undefined" "OverrideRootScale" null null)
  (`self.StartSpawningHighwayCars`))

(event `Daytime1`
  ;[1 0.5664 0] Daytimes
  ;;[1 1 1] Day Start
  (bind _returnvalue (`GameplayStatics.GetActorOfClass` "/Engine/EngineSky/BP_Sky_Sphere.BP_Sky_Sphere_C"))
  (set `self.LightPos` (`/Engine/EngineSky/BP_Sky_Sphere.LightPos1` _returnvalue)))

(event `self.ReceiveTick`
  (params (DeltaSeconds :type "Float (single-precision)"))
  (bind _lightpos (`self.LightPos`))
  (bind _returnvalue (`GameplayStatics.GetActorOfClass` "/Engine/EngineSky/BP_Sky_Sphere.BP_Sky_Sphere_C"))
  (`/Engine/EditorBlueprintResources/StandardMacros.IsValid` _lightpos
    (:`Is Valid`
      (`self.K2_SetActorRotation` _returnvalue (`KismetMathLibrary.RInterpTo` (`self.K2_GetActorRotation` _returnvalue) (`self.K2_GetActorRotation` _lightpos) DeltaSeconds 0.5) false))))

(event `Daytime2`
  ;[1 0.5664 0] Daytimes
  ;;[1 1 1] Client 1 Spawn
  (bind _returnvalue (`GameplayStatics.GetActorOfClass` "/Engine/EngineSky/BP_Sky_Sphere.BP_Sky_Sphere_C"))
  (set `self.LightPos` (`/Engine/EngineSky/BP_Sky_Sphere.LightPos2` _returnvalue)))

(event `Daytime3`
  ;[1 0.5664 0] Daytimes
  ;;[1 1 1] Client 2 Spawn
  (bind _returnvalue (`GameplayStatics.GetActorOfClass` "/Engine/EngineSky/BP_Sky_Sphere.BP_Sky_Sphere_C"))
  (set `self.LightPos` (`/Engine/EngineSky/BP_Sky_Sphere.LightPos3` _returnvalue)))

(event `Daytime4`
  ;[1 0.5664 0] Daytimes
  ;;[1 1 1] Client 3 Spawn
  (bind _returnvalue (`GameplayStatics.GetActorOfClass` "/Engine/EngineSky/BP_Sky_Sphere.BP_Sky_Sphere_C"))
  (set `self.LightPos` (`/Engine/EngineSky/BP_Sky_Sphere.LightPos4` _returnvalue)))

(event `self.ReceiveBeginPlay`
  (bind _returnvalue (`GameplayStatics.GetActorOfClass` "/Engine/EngineSky/BP_Sky_Sphere.BP_Sky_Sphere_C"))
  (set `self.SkySphere` _returnvalue)
  (`self.CreateTutorialUI`)
  (`KismetSystemLibrary.PrintString` (`KismetStringLibrary.BuildString_Name` "" "Initializing: " (`KismetStringLibrary.Conv_StringToName` (`KismetSystemLibrary.GetDisplayName` self))))
  (set `/Game/Gulp/Blueprints/DayCount_BP.Day` (`self.Day`) (`self.DayCountWidget`))
  (`self.SpawnCar`)
  (`self.StartSpawningHighwayCars`))

(event `Daytime5`
  ;[1 0.5664 0] Daytimes
  ;;[1 1 1] Day End
  (bind _returnvalue (`GameplayStatics.GetActorOfClass` "/Engine/EngineSky/BP_Sky_Sphere.BP_Sky_Sphere_C"))
  (set `self.LightPos` (`/Engine/EngineSky/BP_Sky_Sphere.LightPos5` _returnvalue)))

(event `SpawnClient`
  (switch `int` (`self.DispatchedClients`)
    (:`0`
      (`self.Daytime2`))
    (:`1`
      (`self.Daytime3`))
    (:`2`
      (`self.Daytime4`)))
  (bind _returnvalue (`GameplayStatics.GetActorOfClass` "/Game/Gulp/Blueprints/SpawnClientLocation.SpawnClientLocation_C"))
  (`|SpawnActorFromClass` "/Game/Gulp/Blueprints/Client_BP.Client_BP_C" (`KismetMathLibrary.MakeTransform` (`self.K2_GetActorLocation` _returnvalue)) "Undefined" "OverrideRootScale" null null)
  (`KismetSystemLibrary.PrintString` "New Client Spawned"))

(event `SpawnCar`
  (bind _returnvalue (`GameplayStatics.GetActorOfClass` "/Game/Gulp/Blueprints/SpawnCarLocation.SpawnCarLocation_C"))
  (`|SpawnActorFromClass` "/Game/Gulp/Blueprints/Car_BP.Car_BP_C" (`KismetMathLibrary.MakeTransform` (`self.K2_GetActorLocation` _returnvalue)) "Undefined" "OverrideRootScale" null null)
  (`KismetSystemLibrary.PrintString` "Car Spawned"))

(event `CheckDispatchedClients`
  (if (== (`self.DispatchedClients`) 3)
    (`KismetSystemLibrary.PrintString` "Day finished" true true (struct :`R` 0.90625 :`G` 0.167393 :`A` 1.0) 5.0)
    (`self.UpdateOverallMood`)
    (`self.Daytime5`)
    (`KismetSystemLibrary.Delay` 2.0)
    (`self.ActivateDayEndUI`)
    (`GameplayStatics.SetGamePaused` true)
    (else
      (`KismetSystemLibrary.PrintString` "Next client..." true true (struct :`R` 0.90625 :`G` 0.167393 :`A` 1.0) 5.0)
      (`KismetSystemLibrary.Delay` 5.0)
      (`self.SpawnCar`))))

(event `UpdateOverallMood`
  (bind _output_get (set `self.OverallMood` (+ (`self.OverallMood`) (`self.DailyMood`)))))

(event `CheckDay`
  (`self.Daytime1`)
  (if (> (`self.Day`) 3)
    (`KismetSystemLibrary.PrintString` "End of Game" true true (struct :`R` 1.0 :`B` 0.01 :`A` 1.0))
    (`KismetSystemLibrary.PrintString` (`KismetStringLibrary.Conv_IntToString` (stale `UpdateOverallMood` _output_get)))
    (else
      (`self.SpawnCar`))))

(fn `UserConstructionScript`
  (`self.CreateDayCountUI`)
  (`self.CreateMoodMeterUI`)
  (`self.CreatePauseButtonUI`))