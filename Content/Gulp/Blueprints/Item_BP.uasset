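; Item actor that tracks when the Client_BP actor overlaps it and exposes its Name through GetName.
; On begin overlap with the first Client_BP found in the world, it sets IsOverlappingClient and registers itself as that client's CollidingItem.
; On end overlap it clears only its own flag, leaving the client's CollidingItem reference in place.
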(event `self.ReceiveActorBeginOverlap`
  (params (OtherActor :type "Actor Object Reference"))
  (bind _returnvalue (`GameplayStatics.GetActorOfClass` "/Game/Gulp/Blueprints/Client_BP.Client_BP_C"))
  (if (== _returnvalue OtherActor)
    (set `self.IsOverlappingClient` true)
    (set `/Game/Gulp/Blueprints/Client_BP.CollidingItem` self _returnvalue)))

(event `self.ReceiveActorEndOverlap`
  (params (OtherActor :type "Actor Object Reference"))
  (bind _returnvalue (`GameplayStatics.GetActorOfClass` "/Game/Gulp/Blueprints/Client_BP.Client_BP_C"))
  (if (== _returnvalue OtherActor)
    (set `self.IsOverlappingClient` false)))

(fn `GetName`
  (returns (Name :type String))
  (return (`self.Name`)))

(fn `UserConstructionScript`)