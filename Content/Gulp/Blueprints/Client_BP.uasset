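; Client actor that makes randomized fuel and item requests, shown on a widget kept facing the camera by a looping short Delay.
; Mood sums a day-scaled random base with dialogue, item and fuel results; dropped items are validated against the requested class.
; When the task timer expires, unfinished tasks lower mood.
; Once all three tasks are complete, the client destroys itself and reports the dispatch to Main_Gamemode_BP.
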(event `self.ReceiveBeginPlay`
  (`self.StartTaskTimer`)
  (`self.RandomizeRequests`)
  (`SceneComponent.SetVisibility` (`self.Widget`) false false)
  (bind _ascamera_pawn_bp (cast `/Game/Gulp/Blueprints/CameraPawn_BP` (`GameplayStatics.GetPlayerPawn` 0)))
  (set `self.As Camera Pawn BP` _ascamera_pawn_bp)
  (`self.FaceCamera`)
  (`self.RandomizeBaseMood`)
  (`self.UpdateMood`)
  (`KismetSystemLibrary.Delay` 3.0)
  (`self.ShowRequest`))

(event `ShowRequest`
  (bind _widget (`self.Widget`))
  ;[1 1 1] ShowRequest
  (bind _asclient_request_bp (cast `/Game/Gulp/Blueprints/ClientRequest_BP` (`WidgetComponent.GetWidget` _widget)))
  (`SceneComponent.SetVisibility` _widget true false)
  (set `/Game/Gulp/Blueprints/ClientRequest_BP.Fuel` (`KismetTextLibrary.Conv_IntToText` (`self.FuelRequest`)) _asclient_request_bp)
  (`self.FindItem`
    (:`Water`
      (set `self.ItemName` "Water")
      (set `/Game/Gulp/Blueprints/ClientRequest_BP.Item` (`self.ItemName`) _asclient_request_bp :!label _label))
    (:`Chips`
      (set `self.ItemName` "Chips")
      (goto _label))
    (:`Chocolate`
      (set `self.ItemName` "Chocolate")
      (goto _label))
    (:`No Item`
      (set `self.ItemName` "")
      (goto _label))
    (:`Faileld to find`
      (`KismetSystemLibrary.PrintString` "Error: ITEM NOT FOUND"))))

(event `RandomizeRequests`
  (bind (_outitem _outindex) (`KismetArrayLibrary.Array_Random` (`self.ItemRequestReferences`)))
  ;[1 1 1] Randomize Requests
  (set `self.FuelRequest` (`KismetArrayLibrary.Array_Random` (`self.FuelRequests`)))
  (set `self.ItemRequest` _outitem)
  (set `self.ItemClassIndex` _outindex)
  (`self.AutoCompleteEmptyRequests`))

(event `UpdateMood`
  ;[1 1 1] UpdateMood
  (set `self.Mood` (+ (`self.DialogueMoodResult`) (`self.ItemMoodResult`) (`self.FuelMoodResult`) (`self.BaseMood`))))

(event `ClientTimerOver`
  ;[1 1 1] Timer Over: Fail unattended tasks
  (`|ExecutionSequence`
    (:`then_0`
      (if (not (`self.IsDialogueCompleted`))
        (set `self.DialogueMoodResult` -1)))
    (:`then_1`
      (if (not (`self.IsItemCompleted`))
        (set `self.ItemMoodResult` -1)))
    (:`then_2`
      (if (not (`self.IsFuelCompleted`))
        (set `self.FuelMoodResult` -1)))
    (:`then_3`
      (set `self.BaseMood` (- (`self.BaseMood`) 1)))
    (:`then_4`
      (`self.UpdateMood`))))

(event `FaceCamera`
  (bind (_returnvalue_roll _returnvalue_pitch _returnvalue_yaw) (`KismetMathLibrary.BreakRotator` (`KismetMathLibrary.FindLookAtRotation` (`self.K2_GetActorLocation`) (`self.K2_GetActorLocation` (`self.As Camera Pawn BP`)))))
  ;[1 1 1] UI/Widget Faces Camera
  (`SceneComponent.K2_SetRelativeRotation` (`self.Widget`) (`KismetMathLibrary.MakeRotator` _returnvalue_roll _returnvalue_pitch _returnvalue_yaw) false false)
  (`KismetSystemLibrary.Delay` 0.001)
  (`self.FaceCamera`))

(event `ValidateItem`
  ;[1 1 1] Validate Dropped Item
  (bind _returnvalue (`GameplayStatics.GetActorOfClass` "/Game/Gulp/Blueprints/Item_BP.Item_BP_C"))
  (if (`/Game/Gulp/Blueprints/Item_BP.IsOverlappingClient` _returnvalue)
    (bind _returnvalue_2 (`GameplayStatics.GetActorOfClass` (`self.ItemRequest`)))
    (if (== _returnvalue_2 (`self.CollidingItem`))
      (bind _output_get (set `self.ItemMoodResult` 1))
      (`KismetSystemLibrary.PrintString` (`KismetStringLibrary.BuildString_Int` "" "Item Result: " _output_get))
      (else
        (bind _output_get_2 (set `self.ItemMoodResult` -1))
        (`KismetSystemLibrary.PrintString` (`KismetStringLibrary.BuildString_Int` "" "Item Result: " _output_get_2))))
    (set `self.IsItemCompleted` true)
    (`self.CheckReadyForDispatch`)))

(event `StartTaskTimer`
  ;[1 1 1] Start Task Timer
  (`KismetSystemLibrary.PrintString` "Task Timer Started")
  (`self.Create Debug Timer UI`)
  (`KismetSystemLibrary.Delay` (`KismetMathLibrary.Conv_IntToDouble` (`self.ClientTime`)))
  (`self.CheckReadyForDispatch`)
  (if (`self.IsReadyForDispatch`)
    (`self.DispatchClient`)
    (else
      (`self.ClientTimerOver`)
      (`KismetSystemLibrary.PrintString` "TIME IS OVER"))))

(event `RandomizeBaseMood`
  ;[1 1 1] Base Mood Based On Day
  (switch `int` (`self.CurrentDay`)
    (:`1`
      (set `self.BaseMood` (`KismetMathLibrary.Conv_Int64ToInt` (`KismetMathLibrary.RandomInteger64InRange` -1 1))))
    (:`2`
      (set `self.BaseMood` (`KismetMathLibrary.Conv_Int64ToInt` (`KismetMathLibrary.RandomInteger64InRange` -2))))
    (:`3`
      (set `self.BaseMood` (`KismetMathLibrary.Conv_Int64ToInt` (`KismetMathLibrary.RandomInteger64InRange` -3 -1))))))

(event `AutoCompleteEmptyRequests`
  ;[1 1 1] Auto Complete
  (if (not (`KismetSystemLibrary.IsValidClass` (`self.ItemRequest`)))
    (set `self.IsItemCompleted` true)))

(event `CheckReadyForDispatch`
  ;[1 1 1] Check Ready for Dispatch Client
  (if (and (`self.IsDialogueCompleted`) (`self.IsItemCompleted`) (`self.IsFuelCompleted`))
    (`KismetSystemLibrary.PrintString` "Client DISPATCHED ")
    (set `self.IsReadyForDispatch` true)
    (`self.DispatchClient`)))

(event `DispatchClient`
  ;[1 1 1] Dispatch Client
  (`self.K2_DestroyActor`)
  (bind _asmain_gamemode_bp (cast `/Game/Gulp/Blueprints/Main_Gamemode_BP` (`GameplayStatics.GetGameMode`))
    (:`then`
      (`/Engine/EditorBlueprintResources/StandardMacros.IncrementInt` (`/Game/Gulp/Blueprints/Main_Gamemode_BP.DispatchedClients` _asmain_gamemode_bp)
        (:`  `
          (`/Game/Gulp/Blueprints/Main_Gamemode_BP.CheckDispatchedClients` _asmain_gamemode_bp))))
    (:`CastFailed`
      (`KismetSystemLibrary.PrintString` "GAMEMODE CAST FAILED"))))

(fn `UserConstructionScript`)