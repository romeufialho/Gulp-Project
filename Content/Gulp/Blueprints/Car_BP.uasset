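; Car actor that drives in along an entry spline, then drives out along an exit spline and destroys itself.
; MoveCar picks the leg from the Arrived flag and finds the Car_Path_Enter or Car_Path_Leave actor in the level.
; A timeline per leg, rate-scaled by TimeToEnd, sets location and rotation along that spline.
; On arrival it sets Arrived and tells Main_Gamemode_BP to spawn a client.
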(event `self.ReceiveBeginPlay`
  (`self.MoveCar`))

(event `MoveCar`
  (if (not (`self.Arrived`))
    (bind _returnvalue (`GameplayStatics.GetActorOfClass` "/Game/Gulp/Blueprints/Car_Path_Enter.Car_Path_Enter_C"))
    (set `self.EnterSplineREF` _returnvalue)
    (`self.Enter`)
    (else
      (bind _returnvalue_2 (`GameplayStatics.GetActorOfClass` "/Game/Gulp/Blueprints/Car_Path_Leave.Car_Path_Leave_C"))
      (set `self.LeaveSplineREF` _returnvalue_2)
      (`self.Leave`))))

(event `Enter`
  (bind _spline (`/Game/Gulp/Blueprints/Car_Path_Enter.Spline` (`self.EnterSplineREF`)))
  (`TimelineComponent.SetPlayRate` (`self.Move1`) (/ 1.0 (`self.Time to end`)))
  (bind (_direction _move_track) (`Timeline|Move1`)
    (:`Update`
      (bind _returnvalue (`KismetMathLibrary.Lerp` 0.0 (`SplineComponent.GetSplineLength` (`/Game/Gulp/Blueprints/Car_Path_Enter.Spline` (`self.EnterSplineREF`))) _move_track))
      (`self.K2_SetActorTransform` (`KismetMathLibrary.MakeTransform` (`SplineComponent.GetLocationAtDistanceAlongSpline` _spline _returnvalue "World") (`SplineComponent.GetRotationAtDistanceAlongSpline` _spline _returnvalue "World")))
      (if (and (== _move_track 1.0) (not (`self.Arrived`)))
        (`KismetSystemLibrary.PrintString` "Car Arrived")
        (set `self.Arrived` true)
        (bind _asmain_gamemode_bp (cast `/Game/Gulp/Blueprints/Main_Gamemode_BP` (`GameplayStatics.GetGameMode`)))
        (`/Game/Gulp/Blueprints/Main_Gamemode_BP.SpawnClient` _asmain_gamemode_bp)))))

(event `Leave`
  (bind _spline (`/Game/Gulp/Blueprints/Car_Path_Leave.Spline` (`self.LeaveSplineREF`)))
  (`TimelineComponent.SetPlayRate` (`self.Move2`) (/ 1.0 (`self.Time to end`)))
  (bind (_direction _move_track) (`Timeline|Move2`)
    (:`Update`
      (bind _returnvalue (`KismetMathLibrary.Lerp` 0.0 (`SplineComponent.GetSplineLength` (`/Game/Gulp/Blueprints/Car_Path_Leave.Spline` (`self.LeaveSplineREF`))) _move_track))
      (`self.K2_SetActorTransform` (`KismetMathLibrary.MakeTransform` (`SplineComponent.GetLocationAtDistanceAlongSpline` _spline _returnvalue "World") (`SplineComponent.GetRotationAtDistanceAlongSpline` _spline _returnvalue "World")))
      (if (and (== _move_track 1.0) (`self.Arrived`))
        (`KismetSystemLibrary.PrintString` "Car Left")
        (set `self.Arrived` false)
        (`self.K2_DestroyActor`)))))

(fn `UserConstructionScript`)