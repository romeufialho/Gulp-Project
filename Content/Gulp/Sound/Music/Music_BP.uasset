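; Music manager Blueprint that switches between the game's music tracks.
; On BeginPlay it creates a 2D sound for every entry in TrackList and plays them all at once muted, then raises the starting index to the music volume.
; ChangeMusicto swaps tracks by muting the current one and unmuting the chosen index, so all tracks keep running, and prints the new track's name.
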(event `self.ReceiveBeginPlay`
  (bind _output (`|GetArrayItem` (`self.MusicReferences`) (`self.IndexMusic`)))
  (for _array_element (`self.TrackList`)
    (bind _returnvalue (`GameplayStatics.CreateSound2D` _array_element 1.0 1.0 0.0 null))
    (`KismetArrayLibrary.Array_Add` (`self.MusicReferences`) _returnvalue)
    (`AudioComponent.SetVolumeMultiplier` _returnvalue 0.0)
    (`AudioComponent.Play` _returnvalue 0.0))
  (`AudioComponent.SetVolumeMultiplier` _output (`self.Music Volume`))
  (set `self.CurrentMusicREf` _output))

(event `Change Music to`
  (params (`Index of song to play` :type Integer))
  (bind _output (`|GetArrayItem` (`self.MusicReferences`) `Index of song to play`))
  (`AudioComponent.SetVolumeMultiplier` (`self.CurrentMusicREf`) 0.0)
  (`AudioComponent.SetVolumeMultiplier` _output (`self.Music Volume`))
  (bind _output_get (set `self.CurrentMusicREf` _output))
  (`KismetSystemLibrary.PrintString` (`KismetStringLibrary.Concat_StrStr` (`KismetSystemLibrary.GetDisplayName` _output_get))))

(fn `UserConstructionScript`)