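; AI car actor that drives itself along the spline of a Car_Path actor found in the level.
; On BeginPlay it grabs that path and starts a timeline with play rate 1/TimeToEnd, so TimeToEnd controls the trip duration.
; Each update maps the timeline's MOVE value to a distance along the spline and sets the car's world location and rotation from it.
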(event `self.ReceiveBeginPlay`
  (bind _returnvalue (`GameplayStatics.GetActorOfClass` "/Game/Gulp/Assets/Carros/Carros/Car_Path.Car_Path_C"))
  (set `self.SplineREF` _returnvalue)
  (`self.MoveObject2`))

(event `MoveObject2`
  (bind _spline (`/Game/Gulp/Assets/Carros/Carros/Car_Path.Spline` (`self.SplineREF`)))
  (`TimelineComponent.SetPlayRate` (`self.Move object 2`) (/ 1.0 (`self.Time to end`)))
  (bind (_direction _move) (`Timeline|Move object 2`)
    (:`Update`
      (bind _returnvalue (`KismetMathLibrary.Lerp` 0.0 (`SplineComponent.GetSplineLength` (`/Game/Gulp/Assets/Carros/Carros/Car_Path.Spline` (`self.SplineREF`))) _move))
      (`self.K2_SetActorTransform` (`KismetMathLibrary.MakeTransform` (`SplineComponent.GetLocationAtDistanceAlongSpline` _spline _returnvalue "World") (`SplineComponent.GetRotationAtDistanceAlongSpline` _spline _returnvalue "World"))))))

(fn `UserConstructionScript`)