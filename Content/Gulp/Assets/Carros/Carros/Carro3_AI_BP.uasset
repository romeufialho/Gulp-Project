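; Carro3_AI_BP is a car actor that drives itself along a spline path in the level.
; On BeginPlay it finds a Car_Path actor with GetActorOfClass and starts the MoveObject3 timeline, with play rate scaled by 1 / TimeToEnd.
; Each update maps the timeline's Move value to a distance along the spline and sets the car's world location and rotation from that point.
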(event `self.ReceiveBeginPlay`
  (bind _returnvalue (`GameplayStatics.GetActorOfClass` "/Game/Gulp/Assets/Carros/Carros/Car_Path.Car_Path_C"))
  (set `self.Spline REF` _returnvalue)
  (`self.MoveObject3`))

(event `MoveObject3`
  (bind _spline (`/Game/Gulp/Assets/Carros/Carros/Car_Path.Spline` (`self.Spline REF`)))
  (`TimelineComponent.SetPlayRate` (`self.Move Object 3`) (/ 1.0 (`self.Time to End`)))
  (bind (_direction _move) (`Timeline|Move Object 3`)
    (:`Update`
      (bind _returnvalue (`KismetMathLibrary.Lerp` 0.0 (`SplineComponent.GetSplineLength` (`/Game/Gulp/Assets/Carros/Carros/Car_Path.Spline` (`self.Spline REF`))) _move))
      (`self.K2_SetActorTransform` (`KismetMathLibrary.MakeTransform` (`SplineComponent.GetLocationAtDistanceAlongSpline` _spline _returnvalue "World") (`SplineComponent.GetRotationAtDistanceAlongSpline` _spline _returnvalue "World"))))))

(fn `UserConstructionScript`)