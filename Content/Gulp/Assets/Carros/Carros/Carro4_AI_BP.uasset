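; Carro4_AI_BP is an AI car that drives itself along a spline path in the level.
; On BeginPlay it finds the Car_Path_Enter actor and stores it as its spline reference.
; A timeline, with play rate scaled by TimeToEnd, lerps distance along the spline and sets the car's world location and rotation to match each update.
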(event `self.ReceiveBeginPlay`
  (bind _returnvalue (`GameplayStatics.GetActorOfClass` "/Game/Gulp/Assets/Carros/Carros/Car_Path_Enter.Car_Path_Enter_C"))
  (set `self.Spline REF` _returnvalue)
  (`self.Move object 4`))

(event `Move object 4`
  (bind _spline (`/Game/Gulp/Assets/Carros/Carros/Car_Path_Enter.Spline` (`self.Spline REF`)))
  (`TimelineComponent.SetPlayRate` (`self.MoveObject4`) (/ 1.0 (`self.Time to end`)))
  (bind (_direction _move) (`Timeline|MoveObject4`)
    (:`Update`
      (bind _returnvalue (`KismetMathLibrary.Lerp` 0.0 (`SplineComponent.GetSplineLength` (`/Game/Gulp/Assets/Carros/Carros/Car_Path_Enter.Spline` (`self.Spline REF`))) _move))
      (`self.K2_SetActorTransform` (`KismetMathLibrary.MakeTransform` (`SplineComponent.GetLocationAtDistanceAlongSpline` _spline _returnvalue "World") (`SplineComponent.GetRotationAtDistanceAlongSpline` _spline _returnvalue "World"))))))

(fn `UserConstructionScript`)